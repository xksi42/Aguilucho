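; Eagle player for the main menu, judging by its name, that flies itself forward every tick and drives the Aguila animation Blueprint.
; Downward pitch builds acceleration up to a cap, otherwise it decays, while steep pitch sets climb and dive flags passed to the animation.
; Separate functions, not called here, nudge height using a downward trace and set world color parameters in a material parameter collection.
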(event `self.ReceiveTick`
  (params (DeltaSeconds :type "Float (single-precision)"))
  ;[0.5098 1 0 1 75] UPDATE TICK
  (`|ExecutionSequence`
    (:`then_0`
      (`self.Forward`))
    (:`then_1`
      (`self.UpdateAnimBools`))
    (:`then_2`
      (`self.UpdateAnimBP`))))

(event `self.ReceiveBeginPlay`
  ;[1 0 0.2902 1 66] BEGIN PLAY
  ;;[1 1 1] Comment
  (bind _asaguila_anim_bp (cast `/Game/Aguila_animBP` (`SkeletalMeshComponent.GetAnimInstance` (`self.SkeletalMesh`))))
  (`/Engine/EditorBlueprintResources/StandardMacros.IsValid` _asaguila_anim_bp
    (:`Is Valid`
      (set `self.As Aguila Anim BP` _asaguila_anim_bp))))

(fn `lockrot`
  (bind (_returnvalue_roll _returnvalue_pitch _returnvalue_yaw) (`KismetMathLibrary.BreakRotator` (`self.K2_GetActorRotation`)))
  (bind (_returnvalue_x _returnvalue_y) (`KismetMathLibrary.BreakVector` (`self.K2_GetActorLocation`)))
  (bind (_currentlocationlock_x _currentlocationlock_y _currentlocationlock_z) (`KismetMathLibrary.BreakVector` (`self.CurrentLocationLOCK`)))
  (bind (_returnvalue_x_2 _returnvalue_y_2 _returnvalue_z) (`KismetMathLibrary.BreakVector` (`SceneComponent.K2_GetComponentLocation` (`self.PivotMesh`))))
  (`|ExecutionSequence`
    (:`then_0`
      (`/Engine/EditorBlueprintResources/StandardMacros.DoOnce` (`self.BloquearRotacion`)
        (:`Completed`
          (set `self.BloquearRotacion` true)
          (set `self.CurrentLocationLOCK` (`SceneComponent.K2_GetComponentLocation` (`self.PivotMesh`))))))
    (:`then_1`
      (`self.K2_SetActorRotation` (`KismetMathLibrary.MakeRotator` _returnvalue_roll 0.0 _returnvalue_yaw))
      (bind _outhit (`KismetSystemLibrary.LineTraceSingle` (`KismetMathLibrary.MakeVector` _returnvalue_x_2 _returnvalue_y_2 _returnvalue_z) (`KismetMathLibrary.MakeVector` _returnvalue_x _returnvalue_y -200.0) "TraceTypeQuery2"))
      (if (< _returnvalue_z (+ (.z (`.ImpactPoint` (`GameplayStatics.BreakHitResult` _outhit))) _currentlocationlock_z 40.0))
        (`self.K2_SetActorLocation` (`KismetMathLibrary.MakeVector` _returnvalue_x_2 _returnvalue_y_2 (+ _returnvalue_z 1.0)))
        (else
          (`self.K2_SetActorLocation` (`KismetMathLibrary.MakeVector` _returnvalue_x_2 _returnvalue_y_2 _returnvalue_z)))))))

(fn `UserConstructionScript`)