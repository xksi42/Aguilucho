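; Animal actor that can be grabbed and dropped, configured as rabbit, turtle or snake by an enum in the construction script.
; On release it simulates physics; on impact it stops, realigns to the surface normal and clears its grabbed state.
; A hard landing, or a non-turtle overlapping a turtle, sets the dead flag `Sec`.
; Tick then swaps in the death material and shows beacon cubes while not grabbed; proximity beacon logic is disconnected.
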(event `Agafadot`
  (set `PrimitiveComponent.bGenerateOverlapEvents` true (`self.collision`)))

(event `self.ReceiveBeginPlay`
  ;[1 1 1 1 75] Beacon
  (bind _outactors (`GameplayStatics.GetAllActorsOfClass` "/Game/Blueprints/volador.volador_C"))
  (set `self.NewVar_0` (`|GetArrayItem` _outactors)))

(event `CustomEvent_1` :!signature `self.OnTakeAnyDamage`
  (params (DamagedActor :type "Actor Object Reference") (Damage :type "Float (double-precision)") (DamageType :type "DamageType Object Reference") (InstigatedBy :type "Controller Object Reference") (DamageCauser :type "Actor Object Reference")))

(event `self.ReceiveTick`
  (params (DeltaSeconds :type "Float (single-precision)"))
  (bind _cube2 (`self.Cube2`))
  (bind _cube1 (`self.Cube1`))
  ;[1 1 1 1 75] Beacon
  (`|ExecutionSequence`
    (:`then_0`
      (if (`self.Agafat`)
        (`SceneComponent.SetVisibility` _cube1 false true :!label _label)
        (`SceneComponent.SetVisibility` _cube2 false false)
        (elif (`self.Sec`)
          (`/Engine/EditorBlueprintResources/StandardMacros.DoOnce` false :!label _label_2
            (:`Completed`
              (`KismetSystemLibrary.Delay` 0.5)
              (`SceneComponent.K2_SetWorldRotation` :`self` _cube1)
              (`SceneComponent.SetVisibility` _cube1 true true)
              (`SceneComponent.SetVisibility` _cube2 true false)))
          (else
            (goto _label)))))
    (:`then_1`
      (`SceneComponent.K2_SetWorldLocation` (`self.collision`) (`SceneComponent.K2_GetComponentLocation` (`self.Animal`)) false false))
    (:`then_2`
      (if (`self.Sec`)
        (`PrimitiveComponent.SetMaterial` (`self.StaticMesh`) 0 "/Game/Materials/Mort.Mort")))))

(event `CustomEvent`
  (params (DeltaSeconds :type "Float (double-precision)"))
  ;[1 1 1 1 47] Aparició beacon per proximitat (TALLAT)
)

(event `Reboot`
  ;[1 1 1 1 75] Beacon
  (goto _label_2 :!via `Reset`))

(event `Mollat`
  ;[1 1 1 1 56] Mollat
  (`KismetSystemLibrary.Delay` 0.5)
  (`PrimitiveComponent.SetSimulatePhysics` (`self.Animal anchor`) true))

(event `Mort`
  ;[1 1 1 1 66] Mort
  (`KismetSystemLibrary.PrintString` "Sec!")
  (`self.K2_DestroyActor`))

(event `self.Animal.OnComponentHit`
  (params (HitComponent :type "PrimitiveComponent Object Reference") (OtherActor :type "Actor Object Reference") (OtherComp :type "PrimitiveComponent Object Reference") (NormalImpulse :type "Vector Structure") (Hit :type "HitResult Structure (by ref)"))
  (bind (_bblockinghit _binitialoverlap _time _distance _location _impactpoint _normal _impactnormal) (`GameplayStatics.BreakHitResult` Hit))
  (bind _animal_anchor (`self.Animal anchor`))
  ;[1 1 1 1 56] Hostia
  (`|ExecutionSequence`
    (:`then_0`
      (if (>= NormalImpulse_Z (`self.Vel kill`))
        (`KismetSystemLibrary.PrintString` "M'he mort!")
        (bind _output_get (set `self.Sec` true))
        (`KismetSystemLibrary.PrintString` "Sec true" _output_get))
      (`KismetSystemLibrary.Delay` 0.001)
      (set `PrimitiveComponent.bGenerateOverlapEvents` true (`self.collision`))
      (`PrimitiveComponent.SetSimulatePhysics` _animal_anchor false)
      (`SceneComponent.K2_SetWorldLocation` (`self.DefaultSceneRoot`) (`SceneComponent.K2_GetComponentLocation` (`self.Animal anchor`)) false false)
      (`SceneComponent.K2_AttachToComponent` _animal_anchor (`self.DefaultSceneRoot`) "None" "SnapToTarget" "KeepRelative" "KeepRelative" true)
      (`SceneComponent.K2_SetRelativeLocation` (`self.Cube1`) (0.0 0.0 379.999969) false false)
      (`SceneComponent.K2_SetRelativeLocationAndRotation` :`self` (`self.Animal anchor`))
      (`KismetSystemLibrary.PrintString` (`KismetStringLibrary.Conv_RotatorToString` (`KismetMathLibrary.MakeRotator` 0.0)))
      (`self.K2_SetActorRotation` (`KismetMathLibrary.Conv_VectorToRotator` _impactnormal))
      (`SceneComponent.K2_SetRelativeRotation` :`self` (`self.Animal`))
      (`self.K2_SetActorLocation` (`KismetMathLibrary.MakeVector` (.x _impactpoint) (.y _impactpoint) (.z _impactpoint)))
      (`SceneComponent.K2_SetRelativeLocationAndRotation` :`self` (`self.Cube1`) :`NewLocation` (32.0 0.0 0.0)))
    (:`then_2`
      (set `self.Agafat` false)
      (`self.Reboot`))))

(event `self.collision.OnComponentBeginOverlap`
  (params (OverlappedComponent :type "PrimitiveComponent Object Reference") (OtherActor :type "Actor Object Reference") (OtherComp :type "PrimitiveComponent Object Reference") (OtherBodyIndex :type Integer) (bFromSweep :type Boolean) (SweepResult :type "HitResult Structure (by ref)"))
  (bind _asanimal (cast `/Game/Blueprints/Animal` OtherActor))
  (if (`self.Tortuga`)
    _
    (elif (`/Game/Blueprints/Animal.Tortuga` _asanimal)
      (set `self.Sec` true))))

(fn `UserConstructionScript`
  (bind _staticmesh (`self.StaticMesh`))
  (switch `/Game/Blueprints/Animals` (`self.Animals enum`)
    (:`NewEnumerator0`
      (`StaticMeshComponent.SetStaticMesh` _staticmesh "/Game/Meshes/Conejo.Conejo")
      (set `self.Conill` true)
      (set `self.Serp` false)
      (set `self.Tortuga` false))
    (:`NewEnumerator1`
      (`StaticMeshComponent.SetStaticMesh` _staticmesh null)
      (set `self.Tortuga` true)
      (set `self.Serp` false)
      (set `self.Conill` false))
    (:`NewEnumerator2`
      (`StaticMeshComponent.SetStaticMesh` _staticmesh "/Game/Meshes/serpiente_pero_bien.serpiente_pero_bien")
      (set `self.Serp` true)
      (set `self.Tortuga` false)
      (set `self.Conill` false))))