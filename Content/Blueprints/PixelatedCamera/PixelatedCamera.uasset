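; Pixelated camera Blueprint that shows a scene capture as a full-viewport widget with a retro, low-framerate look.
; On BeginPlay it looks up a render target from a resolution data table by the selected enum.
; That target feeds a dynamic material with color, saturation and scanline parameters, used as the widget's canvas brush.
; A looping timer calls CaptureScene to throttle framerate; events change or disable the throttle and refresh the filter.
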(event `self.ReceiveBeginPlay`
  ;[1 1 1] Begin Play - Load PixelateScreenWidget
  (bind _returnvalue (`|CreateWidget` "/Game/Blueprints/PixelatedCamera/pixelateScreen_WDG.pixelateScreen_WDG_C"))
  (bind _output_get (set `self.PiexelatedScreen` _returnvalue))
  (`UserWidget.AddToViewport` _output_get 0)
  (bind _returnvalue_2 (`KismetMaterialLibrary.CreateDynamicMaterialInstance` "/Game/Materials/pixelateScreen_IMAT.pixelateScreen_IMAT"))
  (set `self.DMInstance` _returnvalue_2)
  (`self.SetResolution`
    (:`Execute`
      (`self.UpdateResolutionFilter` (`self.Out Row`)
        (:`Execute`
          (`self.EnableFramerate`))))))

(event `EnableFramerateExec`
  (`self.EnableFramerate`))

(event `DisableFramerateExec`
  (`self.DisableFramerate`))

(event `ChangeFramerate`
  (params (`New Framerate` :type Integer) (Execute :type Boolean))
  (set `self.FrameRate` `New Framerate`)
  (if Execute
    (`self.EnableFramerate`)))

(event `UpdateResolution`
  (`self.UpdateResolutionFilter` (`self.Out Row`)))

(fn `CaptureCurrentFrame`
  (`SceneCaptureComponent2D.CaptureScene` (`self.SceneCaptureComponent2D`)))

(fn `UserConstructionScript`
  (locals (NewLocalVar_0 :type "/Game/Blueprints/PixelatedCamera/resolutionTextures_STR Structure")))