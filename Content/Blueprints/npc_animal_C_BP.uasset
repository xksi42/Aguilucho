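; Animal NPC actor that becomes a rabbit, turtle or snake via an enum in the construction script, and can be grabbed and released.
; On impact it stops physics, snaps upright to the surface normal and shows a beacon, which Tick hides while held.
; Hard impacts or overlapping a turtle (non-turtles only) set Sec, the dead state that Tick applies through materials and AnimBPs.
; Wander movement and proximity-beacon logic are disconnected.
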(event `MOVENPC`)

(event `Mort`
  ;[0.04346 1 0 1 75] STATS
  ;;[1 1 1 1 16] Mort
  (`self.K2_DestroyActor`))

(event `SetColisionsTrue`
  ;[0.04346 1 0 1 75] STATS
  ;;[1 1 1] SET COLISIONS
  (set `PrimitiveComponent.bGenerateOverlapEvents` true (`self.collision`)))

(event `Mollat`
  ;[0.04346 1 0 1 75] STATS
  ;;[1 1 1 1 16] Mollat
  (`KismetSystemLibrary.Delay` 0.5)
  (`PrimitiveComponent.SetSimulatePhysics` (`self.Animal anchor`) true))

(event `self.ReceiveTick`
  (params (DeltaSeconds :type "Float (single-precision)"))
  ;[0.5098 1 0 1 75] EVENT TICK
  (`|ExecutionSequence`
    (:`then_0`
      (if (`self.Agafat`)
        (`SceneComponent.SetVisibility` (`self.BeconPivot`) false true :!label _label)
        (`SceneComponent.SetVisibility` (`self.Becon_B`) false false)
        (elif (not (`self.Sec`))
          (goto _label))))
    (:`then_1`
      (`SceneComponent.K2_SetWorldLocation` (`self.collision`) (`SceneComponent.K2_GetComponentLocation` (`self.MainBody`)) false false))
    (:`then_2`
      (`self.SetAnimalMaterials`))))

(event `ActiveBecon`
  (bind _beconpivot (`self.BeconPivot`))
  ;[1 0.8173 0 1 75] APPARENCE
  ;;[1 1 1 1 16] Beacon
  (`KismetSystemLibrary.Delay` 0.1)
  (`SceneComponent.K2_SetWorldRotation` :`self` _beconpivot)
  (`SceneComponent.SetVisibility` _beconpivot true true)
  (`SceneComponent.SetVisibility` (`self.Becon_B`) true false))

(event `SetAnimalMaterials`
  (bind _sec (`self.Sec`))
  (bind _skeletalmesh (`self.SkeletalMesh`))
  ;[1 0.8173 0 1 75] APPARENCE
  ;;[1 1 1] SET ANIMAL MATERIALS
  (if (`self.Sec`)
    (if (`self.Tortuga`)
      (`PrimitiveComponent.SetMaterial` (`self.StaticMesh`) 0 "/Game/Materials/Mort.Mort")
      (elif (`self.Serp`)
        (`PrimitiveComponent.SetMaterial` _skeletalmesh 0 "/Game/Materials/Mort.Mort")
        (`/Game/Meshes/Serp/Serp_AnimBP.Serp_Anim` (`self.As Serp Anim BP`) _sec false)
        (else
          (`PrimitiveComponent.SetMaterial` _skeletalmesh 0 "/Game/Materials/Mort.Mort")
          (`/Game/Meshes/Conill/Rabbit_AnimBP.Conill_Anim` (`self.As Rabbit Anim BP`) _sec))))))

(event `self.ReceiveBeginPlay`
  (bind _returnvalue (`SkeletalMeshComponent.GetAnimInstance` (`self.SkeletalMesh`)))
  ;[1 0 0.2902 1 75] BEGIN PLAY
  (`|ExecutionSequence`
    (:`then_0`
      (bind _outactors (`GameplayStatics.GetAllActorsOfClass` "/Game/Blueprints/main_player_BP.main_player_BP_C"))
      (set `self.Player` (`|GetArrayItem` _outactors))
      (switch `/Game/Blueprints/Animals` (`self.Animals enum`)
        (:`NewEnumerator0`
          (bind _asrabbit_anim_bp (cast `/Game/Meshes/Conill/Rabbit_AnimBP` _returnvalue))
          (set `self.As Rabbit Anim BP` _asrabbit_anim_bp))
        (:`NewEnumerator2`
          (bind _asserp_anim_bp (cast `/Game/Meshes/Serp/Serp_AnimBP` _returnvalue))
          (set `self.As Serp Anim BP` _asserp_anim_bp))))
    (:`then_1`
      (`self.MOVENPC`))))

(event `self.MainBody.OnComponentHit`
  (params (HitComponent :type "PrimitiveComponent Object Reference") (OtherActor :type "Actor Object Reference") (OtherComp :type "PrimitiveComponent Object Reference") (NormalImpulse :type "Vector Structure") (Hit :type "HitResult Structure (by ref)"))
  (bind (_bblockinghit _binitialoverlap _time _distance _location _impactpoint _normal _impactnormal) (`GameplayStatics.BreakHitResult` Hit))
  (bind _animal_anchor (`self.Animal anchor`))
  (bind _animal_anchor_2 (`self.Animal anchor`))
  ;[0 0.1701 1 1 75] INTERACTIONS
  ;;[1 1 1 1 16] Hostia
  (`|ExecutionSequence`
    (:`then_0`
      (if (>= NormalImpulse_Z (`self.Vel kill`))
        (set `self.Sec` true))
      (`KismetSystemLibrary.Delay` 0.001)
      (set `PrimitiveComponent.bGenerateOverlapEvents` true (`self.collision`))
      (`PrimitiveComponent.SetSimulatePhysics` _animal_anchor false)
      (`SceneComponent.K2_SetWorldLocation` _animal_anchor_2 (`SceneComponent.K2_GetComponentLocation` (`self.Animal anchor`)) false false)
      (`SceneComponent.K2_AttachToComponent` _animal_anchor _animal_anchor_2 "None" "SnapToTarget" "KeepRelative" "KeepRelative" true)
      (`SceneComponent.K2_SetRelativeLocation` (`self.BeconPivot`) (0.0 0.0 379.999969) false false)
      (`SceneComponent.K2_SetRelativeLocationAndRotation` :`self` (`self.Animal anchor`))
      (`self.K2_SetActorRotation` (`KismetMathLibrary.Conv_VectorToRotator` _impactnormal))
      (`SceneComponent.K2_SetRelativeRotation` :`self` (`self.MainBody`))
      (`self.K2_SetActorLocation` _impactpoint)
      (`SceneComponent.K2_SetRelativeLocationAndRotation` :`self` (`self.BeconPivot`) :`NewLocation` (32.0 0.0 0.0)))
    (:`then_2`
      (set `self.Agafat` false)
      (`self.ActiveBecon`))))

(event `self.collision.OnComponentBeginOverlap`
  (params (OverlappedComponent :type "PrimitiveComponent Object Reference") (OtherActor :type "Actor Object Reference") (OtherComp :type "PrimitiveComponent Object Reference") (OtherBodyIndex :type Integer) (bFromSweep :type Boolean) (SweepResult :type "HitResult Structure (by ref)"))
  ;[0 0.1701 1 1 75] INTERACTIONS
  ;;[1 1 1] KillAnimal on colision with other
  (bind _asnpc_animal_c_bp (cast `/Game/Blueprints/npc_animal_C_BP` OtherActor))
  (if (`self.Tortuga`)
    _
    (elif (`/Game/Blueprints/npc_animal_C_BP.Tortuga` _asnpc_animal_c_bp)
      (set `self.Sec` true))))

(event `CustomEvent`
  (params (DeltaSeconds :type "Float (double-precision)"))
  ;[1 1 1 1 47] Aparició beacon per proximitat (TALLAT)
)

(fn `UserConstructionScript`
  (bind _staticmesh (`self.StaticMesh`))
  (bind _skeletalmesh (`self.SkeletalMesh`))
  (switch `/Game/Blueprints/Animals` (`self.Animals enum`)
    (:`NewEnumerator0`
      (`StaticMeshComponent.SetStaticMesh` _staticmesh null)
      (`SkinnedMeshComponent.SetSkinnedAssetAndUpdate` _skeletalmesh "/Game/Meshes/Conill/AnimFinal_RabbitJump_01.AnimFinal_RabbitJump_01" true)
      (`SkeletalMeshComponent.SetAnimInstanceClass` _skeletalmesh "/Game/Meshes/Conill/Rabbit_AnimBP.Rabbit_AnimBP_C")
      (`PrimitiveComponent.SetMaterial` (`self.SkeletalMesh`) 0 "/Game/Materials/Conill.Conill")
      (set `self.Conill` true)
      (set `self.Serp` false)
      (set `self.Tortuga` false))
    (:`NewEnumerator1`
      (`StaticMeshComponent.SetStaticMesh` _staticmesh "/Game/Meshes/Tortuga/Tortuga.Tortuga")
      (`SkinnedMeshComponent.SetSkinnedAssetAndUpdate` _skeletalmesh null true)
      (set `self.Tortuga` true)
      (set `self.Serp` false)
      (set `self.Conill` false))
    (:`NewEnumerator2`
      (`StaticMeshComponent.SetStaticMesh` _staticmesh null)
      (`SkinnedMeshComponent.SetSkinnedAssetAndUpdate` _skeletalmesh "/Game/Meshes/Serp/Serpiente_viva.Serpiente_viva" true)
      (`SkeletalMeshComponent.SetAnimInstanceClass` _skeletalmesh "/Game/Meshes/Serp/Serp_AnimBP.Serp_AnimBP_C")
      (`PrimitiveComponent.SetMaterial` (`self.SkeletalMesh`) 0 "/Game/Materials/Serp.Serp")
      (set `self.Serp` true)
      (set `self.Tortuga` false)
      (set `self.Conill` false))))